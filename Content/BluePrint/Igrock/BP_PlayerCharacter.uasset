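; BP_PlayerCharacter is the player character Blueprint, linking eating, death and loss events to the HUD's win and loss handling.
; On BeginPlay it caches WBP_HUD from MainPlayerHUD and binds the PlayerLosser dispatcher.
; That dispatcher and OnEventDead trigger the HUD's loss event, while OnEating triggers victory when the food count exactly equals CountWinFoods.
; The WidgetSwap input calls the HUD's visible-widget swap.
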(event `self.ReceiveBeginPlay`
  ;[1 1 1] Логика на победу и поражение
  (bind _asmain_player_hud (cast `MainPlayerHUD` (`PlayerController.GetHUD` (`GameplayStatics.GetPlayerController` 0))))
  (bind _aswbp_hud (cast `/Game/UI/WBP_HUD` (`MainPlayerHUD.Widget` _asmain_player_hud)))
  (set `self.As WBP HUD` _aswbp_hud)
  (add `self.DispatcherPlayerLosser` (delegate `Losser`)))

(event `Losser`
  ;[1 1 1] Логика на победу и поражение
  (`/Game/UI/WBP_HUD.PlayerLossEventDispatcher_Event` (`self.As WBP HUD`)))

(event `InputAction|WidgetSwap`
  (params (Key :type "Key Structure"))
  (bind _as_wbp_hud (`self.As WBP HUD`))
  ;[1 1 1] Переключение победителя
  (:`Pressed`
    (if (`KismetSystemLibrary.IsValid` _as_wbp_hud)
      (`/Game/UI/WBP_HUD.SwapVisibleWidgetIsLife` _as_wbp_hud))))

(event `self.OnEating`
  ;[1 1 1] Логика на победу и поражение
  (bind _returnvalue (`self.GetCountFoods`))
  (if (== _returnvalue (`KismetMathLibrary.Conv_IntToDouble` (`self.CountWinFoods`)))
    (`/Game/UI/WBP_HUD.PlayerWinEventDispatcher` (`self.As WBP HUD`))))

(event `self.OnEventDead`
  (bind _as_wbp_hud (`self.As WBP HUD`))
  ;[1 1 1] Логика на победу и поражение
  (if (`KismetSystemLibrary.IsValid` _as_wbp_hud)
    (`/Game/UI/WBP_HUD.PlayerLossEventDispatcher_Event` _as_wbp_hud)))

(fn `UserConstructionScript`)