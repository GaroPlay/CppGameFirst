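; BP_Red_Bird is a Paper2D flipbook enemy that repeatedly fires scaled-down BP_Shot_Fire projectiles from a spawn point.
; A self-calling Shot event, started at BeginPlay, spawns and delays while ShotRight is true.
; Any overlap on KillSelf kills it: the death flipbook plays, collision turns off, shooting stops and a short lifespan removes it.
; Fly is an empty stub for a planned Y-axis patrol.
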(event `self.ReceiveBeginPlay`
  (`self.Shot`))

(event `Shot`
  ;[1 1 1] Comment
  (if (`self.ShotRight`)
    (`|SpawnActorFromClass` "/Game/BluePrints/Charactar/Enemy/RedBird/BP_Shot_Fire.BP_Shot_Fire_C" (`KismetMathLibrary.MakeTransform` (`SceneComponent.K2_GetComponentLocation` (`self.Point_Start_Shot`)) (`KismetMathLibrary.MakeRotator` 0.0 (`self.Rotation_Y_(Pitch)_Shot`)) (0.5 0.5 0.5)) "AlwaysSpawn" "OverrideRootScale" self null)
    (`KismetSystemLibrary.Delay` (`self.Shot_Delation`))
    (`self.Shot`)))

(event `self.KillSelf.OnComponentBeginOverlap`
  (params (OverlappedComponent :type "PrimitiveComponent Object Reference") (OtherActor :type "Actor Object Reference") (OtherComp :type "PrimitiveComponent Object Reference") (OtherBodyIndex :type Integer) (bFromSweep :type Boolean) (SweepResult :type "HitResult Structure (by ref)"))
  ;[1 1 1] Смерть самого NPC
  (`PaperFlipbookComponent.SetFlipbook` (`self.PaperFlipbook`) "/Game/Assets/Props_Items_and_VFX/fireball-hit/Sprites/FB_Fireball_Dead.FB_Fireball_Dead")
  (`PrimitiveComponent.SetCollisionEnabled` (`self.KillSelf`) "NoCollision")
  (set `self.ShotRight` false)
  (`self.SetLifeSpan` 0.5))

(event `Fly`
  ;[1 1 1] Тут надо реализовать зону патрулирования в оси Y
)

(fn `UserConstructionScript`)