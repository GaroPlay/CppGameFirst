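; BP_Shot_Fire is the RedBird enemy's fireball projectile, which damages the player on contact and expires after a short lifetime.
; Tick plays the MoveShot timeline, whose update subtracts an AddAxxisX offset from the actor's location without sweeping.
; The first FireKill overlap, noted as Pawn-only, shortens the lifespan and sends hurt-flipbook, kill and health-subtraction messages to the overlapped actor.
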(event `self.ReceiveBeginPlay`
  ;[1 1 1 1 12] Уничтожаем шар по времени
  (`self.SetLifeSpan` 3.0))

(event `ShotMove`
  ;[1 1 1] Тут движения огненого шара
  (bind (_direction _alpha _add_axxis_x) (`Timeline|MoveShot`)
    (:`Update`
      (`self.K2_SetActorLocation` (- (`self.K2_GetActorLocation`) _add_axxis_x)))))

(event `self.ReceiveTick`
  (params (DeltaSeconds :type "Float (single-precision)"))
  ;[1 1 1] Тут движения огненого шара
  (`self.ShotMove`))

(event `self.FireKill.OnComponentBeginOverlap`
  (params (OverlappedComponent :type "PrimitiveComponent Object Reference") (OtherActor :type "Actor Object Reference") (OtherComp :type "PrimitiveComponent Object Reference") (OtherBodyIndex :type Integer) (bFromSweep :type Boolean) (SweepResult :type "HitResult Structure (by ref)"))
  ;[1 1 1] Колизия настроена на перекрытие только Pawns
  ;;[1 1 1] Урон игроку от огненного шара
  (`/Engine/EditorBlueprintResources/StandardMacros.DoOnce` false
    (:`Completed`
      (`self.SetLifeSpan` 0.15)
      ;;;[1 1 1 1 14] Вызываем анимацию попадения
      (message `/Game/BluePrints/Interface/BPI_Kill.Shot_Hurt_FlipBook` OtherActor)
      (message `/Game/BluePrints/Interface/BPI_Kill.Kill_Player_Pawn` OtherActor)
      (message `/Game/BluePrints/Interface/BPI_Gem_And_Healt.SubstractHealPlayerPawn` OtherActor))))

(fn `UserConstructionScript`)