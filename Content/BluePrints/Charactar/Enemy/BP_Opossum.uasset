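; BP_Opossum is a 2D Paper2D enemy that patrols back and forth between its spawn point and a TargetPoint.
; A ping-pong timeline lerps its position, with play rate scaled by path distance for constant speed.
; The flipbook yaw follows travel direction.
; KillPlayerBox overlaps send kill and health-loss messages to the other actor, while KillSelfBox overlaps play death, disable both boxes and expire the opossum.
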(event `self.ReceiveBeginPlay`
  ;[1 1 1 1 12] Начальная и конечная точка пути
  (`self.InitLocations`)
  ;[1 1 1 1 12] Задаем индивидуально скорость для экземпляра
  (`self.SetPlayRate`)
  ;[1 1 1 1 12] Определяе сторону передвижения
  (`self.InitMovingLeft`)
  (`self.MoveToEnd `))

(event `MoveToEnd`
  ;[1 1 1] Тут планое движение от (Start к End)
  (bind (_direction _alpha) (`Timeline|Move` :!label _label)
    (:`Update`
      (`self.K2_SetActorLocation` (`KismetMathLibrary.VLerp` (`self.StartLocation`) (`self.EndLocation`) _alpha)))
    (:`Finished`
      ;;[1 1 1 1 14] Мы тут разворачиаем Sprate при каждом окончание пути
      (set `self.B_Is_Move_Left` (not (`self.B_Is_Move_Left`)))
      ;;[1 1 1] Зацикливание Time line Стандарт
      (switch `ETimelineDirection` _direction
        (:`Forward`
          (`self.MoveToStart`))
        (:`Backward`
          (`self.MoveToEnd `))))))

(event `MoveToStart`
  ;[1 1 1] Тут планое движение от (Start к End)
  (goto _label :!via `Reverse`))

(event `UpdateRotateAnimation`
  ;[1 1 1] Обновление повора
  (`SceneComponent.K2_SetRelativeRotation` (`self.PaperFlipbook`) (`KismetMathLibrary.MakeRotator` 0.0 0.0 (`KismetMathLibrary.SelectFloat` 0.0 180.0 (`self.B_Is_Move_Left`))) false false))

(event `self.ReceiveTick`
  (params (DeltaSeconds :type "Float (single-precision)"))
  (`self.UpdateRotateAnimation`))

(event `self.KillSelfBox.OnComponentBeginOverlap`
  (params (OverlappedComponent :type "PrimitiveComponent Object Reference") (OtherActor :type "Actor Object Reference") (OtherComp :type "PrimitiveComponent Object Reference") (OtherBodyIndex :type Integer) (bFromSweep :type Boolean) (SweepResult :type "HitResult Structure (by ref)"))
  ;[1 1 1] Cмерть самого NPC
  (`PaperFlipbookComponent.SetFlipbook` (`self.PaperFlipbook`) "/Game/Assets/Props_Items_and_VFX/Sunnyland_FX/Sprites/enemy-death/FB_Enemy-death.FB_Enemy-death")
  (`PrimitiveComponent.SetCollisionEnabled` (`self.KillPlayerBox`) "NoCollision")
  (`PrimitiveComponent.SetCollisionEnabled` (`self.KillSelfBox`) "NoCollision")
  (`self.SetLifeSpan` 0.5))

(event `self.KillPlayerBox.OnComponentBeginOverlap`
  (params (OverlappedComponent :type "PrimitiveComponent Object Reference") (OtherActor :type "Actor Object Reference") (OtherComp :type "PrimitiveComponent Object Reference") (OtherBodyIndex :type Integer) (bFromSweep :type Boolean) (SweepResult :type "HitResult Structure (by ref)"))
  ;[1 1 1] Тут вызывам Kill у игрока если он столкнулся с NPC
  (message `/Game/BluePrints/Interface/BPI_Kill.Kill_Player_Pawn` OtherActor)
  (message `/Game/BluePrints/Interface/BPI_Gem_And_Healt.SubstractHealPlayerPawn` OtherActor))

(fn `InitLocations`
  (set `self.StartLocation` (`self.K2_GetActorLocation`))
  (set `self.EndLocation` (`SceneComponent.K2_GetComponentLocation` (`self.TargetPoint`)))
  (return))

(fn `InitMovingLeft`
  (bind _startlocation_x (`KismetMathLibrary.BreakVector` (`self.StartLocation`)))
  (bind _endlocation_x (`KismetMathLibrary.BreakVector` (`self.EndLocation`)))
  (set `self.B_Is_Move_Left` (> (- _startlocation_x _endlocation_x) 0.0))
  (return))

(fn `SetPlayRate`
  (`TimelineComponent.SetPlayRate` (`self.Move`) (/ (`self.Speed(relation)`) (`KismetMathLibrary.Vector_Distance` (`self.StartLocation`) (`self.EndLocation`))))
  (return))

(fn `UserConstructionScript`
  (`SceneComponent.K2_SetRelativeLocation` (`self.TargetPoint`) (`self.EndLocation`) false false))